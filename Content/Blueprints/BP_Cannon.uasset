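; BP_Cannon is a destructible turret actor that shoots at the player whenever it has line of sight.
; Each Tick it traces from its Sphere to the player and, if the hit is BP_Dude, rotates to face them.
; A Delay on that Tick path throttles BP_CannonProjectile spawns at the Sphere's transform to roughly one per second.
; Each TakeDamage event removes one life regardless of damage amount, destroying the cannon at zero.
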(event Custom|TakeDamage
  (bind _output_get (Variables|Default|SetLives (- (Variables|Default|GetLives) 1.0)))
  (if (<= _output_get 0.0)
    (Actor|DestroyActor)))

(event EventBeginPlay)

(event Collision|EventActorBeginOverlap
  (params (OtherActor :type Actor%20Object%20Reference)))

(event EventTick
  (params (DeltaSeconds :type Float%20%28single-precision%29))
  (bind _returnvalue (Game|GetPlayerCharacter 0))
  (bind _returnvalue_2 (Transformation|GetActorLocation _returnvalue))
  (bind _outhit (Collision|LineTraceByChannel (Transformation|GetWorldLocation (Variables|Default|GetSphere)) _returnvalue_2 "TraceTypeQuery1" false 0 "ForOneFrame"))
  (Utilities|Casting|CastToBP_Dude (.HitActor (Collision|BreakHitResult _outhit)))
  (Transformation|SetActorRotation (Math|Rotator|FindLookatRotation (Transformation|GetActorLocation) _returnvalue_2))
  (Utilities|FlowControl|Delay 1.0)
  (Game|SpawnActorfromClass "/Game/Blueprints/BP_CannonProjectile.BP_CannonProjectile_C" (Transformation|GetWorldTransform (Variables|Default|GetSphere)) "Undefined" "MultiplyWithRoot" 0 0))

(fn ConstructionScript)