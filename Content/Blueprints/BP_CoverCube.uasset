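; BP_CoverCube is an interactable cover prop that uses a riot shield mesh.
; Its construction script sets the mesh and, for one specific InteractionType value, turns on physics simulation with the PhysicsBody collision type.
; GetInteractionType exposes that type to callers, while OnInteract is only a stub that prints a debug message.
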(event EventBeginPlay)

(event Collision|EventActorBeginOverlap
  (params (OtherActor :type Actor%20Object%20Reference)))

(event EventTick
  (params (DeltaSeconds :type Float%20%28single-precision%29)))

(event EventOnInteract
  (Development|PrintString "Interacting"))

(fn ConstructionScript
  (Components|StaticMesh|SetStaticMesh (Variables|Default|GetcoverCube) "/Game/Fab/Riot_Shield/riot_shield/StaticMeshes/RiotShield.RiotShield")
  (if (Utilities|Enum|Equal(Enum) (Variables|Default|GetInteractionType) "NewEnumerator1")
    (Physics|SetSimulatePhysics (Variables|Default|GetcoverCube) true)
    (Collision|SetCollisionObjectType (Variables|Default|GetcoverCube) "ECC_PhysicsBody")))

(fn GetInteractionType
  (return (Variables|Default|GetInteractionType)))